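; BP_ItemBase is a base pickup item that a player can grab into their hand through an Interact event.
; On interaction it copies its mesh, first material and world scale onto the player's ItemPlace component.
; It records the scale and its own class on the player as ItemScale and SpawnItem, destroys itself, and sets the player's InHand flag.
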(event `self.ReceiveTick`
  (params (DeltaSeconds :type "Float (single-precision)")))

(event `self.ReceiveBeginPlay`)

(event `/Game/Blueprints/BP_Interface.Interact`
  (params (InteractActor :type "/Game/Blueprints/BP_Player Object Reference"))
  (bind _objectmesh (`self.ObjectMesh`))
  (bind _itemplace (`/Game/Blueprints/BP_Player.ItemPlace` (`self.Player`)))
  (bind _output_get (set `self.Player` InteractActor))
  (`StaticMeshComponent.SetStaticMesh` (`/Game/Blueprints/BP_Player.ItemPlace` _output_get) (`StaticMeshComponent.StaticMesh` _objectmesh))
  (`PrimitiveComponent.SetMaterial` _itemplace 0 (`PrimitiveComponent.GetMaterial` _objectmesh 0))
  (bind _output_get_2 (set `/Game/Blueprints/BP_Player.ItemScale` (`SceneComponent.K2_GetComponentScale` (`self.ObjectMesh`)) (`self.Player`)))
  (`SceneComponent.SetWorldScale3D` _itemplace _output_get_2)
  (set `/Game/Blueprints/BP_Player.SpawnItem` (`GameplayStatics.GetObjectClass` self) (`self.Player`))
  (`self.K2_DestroyActor`)
  (set `/Game/Blueprints/BP_Player.InHand` true (`self.Player`)))

(fn `UserConstructionScript`)
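; Player Blueprint that adds a crosshair widget on BeginPlay and handles left-click interaction and dropping of a held item.
; With empty hands, a click line-traces from FollowCamera on the Visibility channel and sends the Interact interface message to the hit actor, passing itself.
; With an item in hand, a click clears the ItemPlace mesh, spawns SpawnItem there at ItemScale and resets InHand, provided SpawnItem is valid.
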(event `self.ReceiveBeginPlay`
  (bind _returnvalue (`|CreateWidget` "/Game/Blueprints/HUD/WBP_Crosshair.WBP_Crosshair_C"))
  (`UserWidget.AddToPlayerScreen` _returnvalue 0))

(event `Key|LeftMouseButton`
  (params (Key :type "Key Structure"))
  (bind _followcamera (`self.FollowCamera`))
  (bind _returnvalue (`SceneComponent.K2_GetComponentLocation` _followcamera))
  (bind (_returnvalue_location _returnvalue_rotation) (`KismetMathLibrary.BreakTransform` (`SceneComponent.K2_GetComponentToWorld` (`self.ItemPlace`))))
  (:`Pressed`
    (if (`self.InHand`)
      (`self.SpawnItem`
        (:`then`
          (`StaticMeshComponent.SetStaticMesh` (`self.ItemPlace`) null)
          (`|SpawnActorFromClass` (`self.SpawnItem`) (`KismetMathLibrary.MakeTransform` _returnvalue_location _returnvalue_rotation (`self.ItemScale`)) "Undefined" "OverrideRootScale" null null)
          (set `self.InHand` false))
        (:`else`))
      (else
        (bind (_outhit _returnvalue_2) (`KismetSystemLibrary.LineTraceSingle` _returnvalue (+ _returnvalue (* (`KismetMathLibrary.GetForwardVector` (`SceneComponent.K2_GetComponentRotation` _followcamera)) (`self.LineTraceDistance`))) "TraceTypeQuery1"))
        (if _returnvalue_2
          (message `/Game/Blueprints/BP_Interface.Interact` (`.HitActor` (`GameplayStatics.BreakHitResult` _outhit)) self))))))

(fn `UserConstructionScript`)